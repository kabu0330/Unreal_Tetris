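; Falling Tetris piece actor that lands on static geometry and then spawns the next piece.
; The construction script randomly picks one of seven tetromino shapes, arranging four cubes by local offsets and tinting their materials.
; A looping timer moves the actor down one cell per tick while short downward WorldStatic traces from each child component check for support.
; On a hit, it stops the timer and spawns a new BP_Tetromino at a fixed height.
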(event `self.ReceiveBeginPlay`
  (bind _returnvalue (`KismetSystemLibrary.K2_SetTimerDelegate` (delegate `DropEvent`) (`self.DropSpeedTime`) true))
  (set `self.TimerHandle` _returnvalue))

(event `DropEvent`
  (set `self.bIsDropping` true)
  (for _array_element (`SceneComponent.GetChildrenComponents` (`self.SceneComponent`) false)
    (bind _returnvalue (`SceneComponent.K2_GetComponentLocation` _array_element))
    (bind (_outhit _returnvalue_2) (`KismetSystemLibrary.LineTraceSingleForObjects` _returnvalue (- _returnvalue (0.0 0.0 50.0)) (`|MakeArray` "ObjectTypeQuery1" :!type "EObjectTypeQuery Enum")))
    (if _returnvalue_2
      (`/Engine/EditorBlueprintResources/StandardMacros.DoOnce` false
        (:`Completed`
          (set `self.bIsDropping` false)
          (`KismetSystemLibrary.K2_ClearAndInvalidateTimerHandle` (`self.TimerHandle`))))))
  (if (`self.bIsDropping`)
    (`self.K2_AddActorLocalOffset` (0.0 0.0 -100.0))
    (else
      (`|SpawnActorFromClass` "BP_Tetromino_C" (`KismetMathLibrary.MakeTransform` (0.0 0.0 1000.0)) "Undefined" "MultiplyWithRoot" null null))))

(fn `UserConstructionScript`
  (switch `int` (`KismetMathLibrary.RandomIntegerInRange` 0 6)
    (:`0`
      ; I Tetromino
      (`SceneComponent.K2_AddLocalOffset` (`self.Cube2`) (0.0 0.0 100.0) false false)
      (`SceneComponent.K2_AddLocalOffset` (`self.Cube3`) (0.0 0.0 200.0) false false)
      (`SceneComponent.K2_AddLocalOffset` (`self.Cube4`) (0.0 0.0 300.0) false false)
      (set `self.BlockColor` (struct :`R` 0.039 :`G` 0.517 :`B` 0.89 :`A` 1.0)))
    (:`1`
      ; L Tetromino
      (`SceneComponent.K2_AddLocalOffset` (`self.Cube2`) (0.0 0.0 100.0) false false)
      (`SceneComponent.K2_AddLocalOffset` (`self.Cube3`) (0.0 0.0 200.0) false false)
      (`SceneComponent.K2_AddLocalOffset` (`self.Cube4`) (0.0 100.0 0.0) false false)
      (set `self.BlockColor` (struct :`R` 1.0 :`G` 0.949 :`A` 1.0)))
    (:`2`
      ; S Tetromino
      (`SceneComponent.K2_AddLocalOffset` (`self.Cube2`) (0.0 0.0 100.0) false false)
      (`SceneComponent.K2_AddLocalOffset` (`self.Cube3`) (0.0 100.0 100.0) false false)
      (`SceneComponent.K2_AddLocalOffset` (`self.Cube4`) (0.0 100.0 200.0) false false)
      (set `self.BlockColor` (struct :`R` 1.0 :`G` 0.226567 :`B` 0.813676 :`A` 1.0)))
    (:`3`
      ; Z Tetromino
      (`SceneComponent.K2_AddLocalOffset` (`self.Cube2`) (0.0 0.0 100.0) false false)
      (`SceneComponent.K2_AddLocalOffset` (`self.Cube3`) (0.0 -100.0 100.0) false false)
      (`SceneComponent.K2_AddLocalOffset` (`self.Cube4`) (0.0 -100.0 200.0) false false)
      (set `self.BlockColor` (struct :`R` 0.137812 :`G` 0.185213 :`B` 0.98 :`A` 1.0)))
    (:`4`
      ; T Tetromino
      (`SceneComponent.K2_AddLocalOffset` (`self.Cube2`) (0.0 -100.0 0.0) false false)
      (`SceneComponent.K2_AddLocalOffset` (`self.Cube3`) (0.0 100.0 0.0) false false)
      (`SceneComponent.K2_AddLocalOffset` (`self.Cube4`) (0.0 0.0 100.0) false false)
      (set `self.BlockColor` (struct :`R` 0.624 :`G` 0.091 :`B` 0.111348 :`A` 1.0)))
    (:`5`
      ; O Tetromino
      (`SceneComponent.K2_AddLocalOffset` (`self.Cube2`) (0.0 0.0 100.0) false false)
      (`SceneComponent.K2_AddLocalOffset` (`self.Cube3`) (0.0 100.0 0.0) false false)
      (`SceneComponent.K2_AddLocalOffset` (`self.Cube4`) (0.0 100.0 100.0) false false)
      (set `self.BlockColor` (struct :`R` 0.157604 :`G` 0.89 :`B` 0.416 :`A` 1.0)))
    (:`6`
      ; J Tetromino
      (`SceneComponent.K2_AddLocalOffset` (`self.Cube2`) (0.0 0.0 100.0) false false)
      (`SceneComponent.K2_AddLocalOffset` (`self.Cube3`) (0.0 0.0 200.0) false false)
      (`SceneComponent.K2_AddLocalOffset` (`self.Cube4`) (0.0 -100.0 0.0) false false)
      (set `self.BlockColor` (struct :`R` 1.0 :`G` 0.509367 :`B` 0.041667 :`A` 1.0))))
  (`MeshComponent.SetVectorParameterValueOnMaterials` (`self.Cube1`) "Color" (`KismetMathLibrary.Conv_LinearColorToVector` (`self.BlockColor`)))
  (`MeshComponent.SetVectorParameterValueOnMaterials` (`self.Cube2`) "Color" (`KismetMathLibrary.Conv_LinearColorToVector` (`self.BlockColor`)))
  (`MeshComponent.SetVectorParameterValueOnMaterials` (`self.Cube3`) "Color" (`KismetMathLibrary.Conv_LinearColorToVector` (`self.BlockColor`)))
  (`MeshComponent.SetVectorParameterValueOnMaterials` (`self.Cube4`) "Color" (`KismetMathLibrary.Conv_LinearColorToVector` (`self.BlockColor`))))