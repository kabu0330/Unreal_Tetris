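; Line-clear checker actor for a falling-block puzzle, Tetris-style, with all logic in CheckLines.
; Box components act as row sensors, each counting overlapping BP_SingleBlock actors to detect full rows of ten.
; Each full row increases DropAmount; those below CutoffLineZ also lower that cutoff and have their blocks exploded and destroyed.
; A final pass shifts gathered actors lying below the cutoff down by DropAmount.
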(fn `CheckLines`
  (locals (OverlapingAcotrs :type "Array of Actor Object Reference") (DropAmount :type "Float (double-precision)") (CutoffLineZ :type "Float (double-precision)"))
  (for _array_element (`|MakeArray` (`self.GetComponentByClass` "/Script/Engine.BoxComponent"))
    (set `local.OverlapingAcotrs` (`PrimitiveComponent.GetOverlappingActors` _array_element "/Game/Blueprint/BP_SingleBlock.BP_SingleBlock_C"))
    (if (== (`KismetArrayLibrary.Array_Length` (`local.OverlapingAcotrs`)) 10)
      (set `local.DropAmount` (+ (`local.DropAmount`) 50.0))
      (bind (_returnvalue_x _returnvalue_y _returnvalue_z) (`KismetMathLibrary.BreakVector` (`SceneComponent.K2_GetComponentLocation` _array_element)))
      (if (< _returnvalue_z (`local.CutoffLineZ`))
        (set `local.CutoffLineZ` _returnvalue_z)
        (for _array_element_2 (`local.OverlapingAcotrs`)
          (`GameplayStatics.SpawnEmitterAtLocation` "/Game/StarterContent/Particles/P_Explosion.P_Explosion" (`self.K2_GetActorLocation` _array_element_2))
          (`self.K2_DestroyActor` _array_element_2)))))
  (bind _outactors (`GameplayStatics.GetAllActorsOfClass` null))
  (for _array_element_3 _outactors
    (bind (_returnvalue_x_2 _returnvalue_y_2 _returnvalue_z_2) (`KismetMathLibrary.BreakVector` (`self.K2_GetActorLocation` _array_element_3)))
    (if (< _returnvalue_z_2 (`local.CutoffLineZ`))
      (`self.K2_SetActorLocation` _array_element_3 (`KismetMathLibrary.MakeVector` _returnvalue_x_2 _returnvalue_y_2 (- _returnvalue_z_2 (`local.DropAmount`))) false false))))

(fn `UserConstructionScript`)